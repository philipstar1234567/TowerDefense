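; Old grid manager actor that builds a rectangular tile grid at BeginPlay for placement, with a build mode view of occupied and free tiles.
; GenerateGrid adds one instanced mesh per tile and stores position, coordinates and instance index in a nested row array.
; SetTileColor writes RGBA into per-instance custom data, which UpdateEveryTileColor uses for red/green or neutral grey.
; GetTileFromWorldPosition converts world positions to bounds-checked tile data.
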(event Custom|GenerateGrid
  (bind _tilesize (Variables|Default|GetTileSize))
  ;[0.15 0.15 0.15 0.5] Grid Generation System (not a mess at all...)
  (Components|InstancedStaticMesh|ClearInstances (Variables|Default|GetTileVisuals))
  (for _index (range 0 (- (Variables|Default|GetGridSizeX) 1))
    (Utilities|Array|Clear (Variables|Default|GetTempRowTiles))
    (for _index_2 (range 0 (- (Variables|Default|GetGridSizeY) 1))
      (bind _returnvalue (Components|InstancedStaticMesh|AddInstance (Variables|Default|GetTileVisuals) (Math|Transform|MakeTransform (+ (Math|Vector|MakeVector (+ (* _index _tilesize) (* _tilesize 0.5)) (+ (* _tilesize _index_2) (* _tilesize 0.5)) 0.0) (Transformation|GetActorLocation)) "0, 0, 0" "1.000000,1.000000,0.100000") true))
      (Utilities|Array|Add (Variables|Default|GetTempRowTiles) (Utilities|Struct|MakeST_TileDataOLD (+ (Math|Vector|MakeVector (+ (* _index _tilesize) (* _tilesize 0.5)) (+ (* _tilesize _index_2) (* _tilesize 0.5)) 0.0) (Transformation|GetActorLocation)) false (Math|Vector2D|MakeVector2D (Math|Conversions|ToFloat(Integer) _index) (Math|Conversions|ToFloat(Integer) _index_2)) _returnvalue)))
    (Utilities|Array|Add (Variables|Default|GetGridArray) (Utilities|Struct|MakeST_TileRowOLD (Variables|Default|GetTempRowTiles)))))

(event Custom|UpdateEveryTileColor
  (params (BuildMode :type Boolean))
  ;[0.15 0.15 0.15 0.5] GiveColorToWholeGrid
  (for _array_element (Variables|Default|GetGridArray)
    (for _array_element_2 (.rowtiles _array_element)
      (if BuildMode
        (if (.isoccupied _array_element_2)
          (CallFunction|SetTileColor (.gridcoord _array_element_2) "(R=1.000000,G=0.000000,B=0.000000,A=1.000000)")
          (else
            (CallFunction|SetTileColor (.gridcoord _array_element_2) "(R=0.000000,G=1.000000,B=0.000000,A=1.000000)")))
        (else
          (CallFunction|SetTileColor (.gridcoord _array_element_2) "(R=0.682292,G=0.682292,B=0.682292,A=1.000000)"))))))

(event EventBeginPlay
  (bind _tilevisuals (Variables|Default|GetTileVisuals))
  ;[0.15 0.15 0.15 0.5] OnBeginPlay
  (Utilities|Array|Clear (Variables|Default|GetGridArray))
  (CallFunction|GenerateGrid)
  (bind _returnvalue (Rendering|Material|CreateDynamicMaterialInstance _tilevisuals 0 (Rendering|Material|GetMaterial _tilevisuals 0) "None" :!class /Script/Engine.PrimitiveComponent))
  (Variables|Default|SetTileMaterial _returnvalue)
  (CallFunction|UpdateEveryTileColor false))

(fn ConstructionScript)

(fn GetTilefromWorldPosition
  (params (WorldPos :type Vector))
  (bind _returnvalue (Transformation|GetActorLocation))
  (bind _tilesize (Variables|Default|GetTileSize))
  (bind _returnvalue_2 (- WorldPos _returnvalue))
  (bind _returnvalue_3 (/ (.x _returnvalue_2) _tilesize))
  (bind _returnvalue_4 (/ (.y _returnvalue_2) _tilesize))
  (bind _returnvalue_5 (Math|Float|Floor _returnvalue_4))
  (bind _returnvalue_6 (Math|Float|Floor _returnvalue_3))
  (if (and (and (and (>= _returnvalue_6 0) (< _returnvalue_6 (Variables|Default|GetGridSizeX))) (>= _returnvalue_5 0)) (< _returnvalue_5 (Variables|Default|GetGridSizeY)))
    (return (Utilities|Array|Get(acopy) (.rowtiles (Utilities|Array|Get(acopy) (Variables|Default|GetGridArray) _returnvalue_6)) _returnvalue_5) true)
    (else
      (return "" false))))

(fn SetTileColor
  (params (GridCoords :type Vector%202D%20Structure) (NewColor :type Linear%20Color%20Structure))
  (bind (_r _g _b _a) (Utilities|Struct|BreakLinearColor NewColor))
  (bind _tilevisuals (Variables|Default|GetTileVisuals))
  (LocalVariables|SetGridX (Math|Float|Floor (.x GridCoords)))
  (LocalVariables|SetGridY (Math|Float|Floor (.y GridCoords)))
  (if (and (and (>= (LocalVariables|GetGridY) 0) (< (LocalVariables|GetGridY) (Variables|Default|GetGridSizeY))) (and (>= (LocalVariables|GetGridX) 0) (< (LocalVariables|GetGridX) (Variables|Default|GetGridSizeX))))
    (Class|InstancedStaticMeshComponent|SetNumCustomDataFloats (Variables|Default|GetTileVisuals) 4)
    (Components|InstancedStaticMesh|SetCustomDataValue _tilevisuals (.InstanceIndex (Utilities|Struct|BreakST_TileDataOLD (Utilities|Array|Get(acopy) (Utilities|Struct|BreakST_TileRowOLD (Utilities|Array|Get(acopy) (Variables|Default|GetGridArray) (LocalVariables|GetGridX))) (LocalVariables|GetGridY)))) 0 _r false)
    (Components|InstancedStaticMesh|SetCustomDataValue _tilevisuals (.InstanceIndex (Utilities|Struct|BreakST_TileDataOLD (Utilities|Array|Get(acopy) (Utilities|Struct|BreakST_TileRowOLD (Utilities|Array|Get(acopy) (Variables|Default|GetGridArray) (LocalVariables|GetGridX))) (LocalVariables|GetGridY)))) 1 _g false)
    (Components|InstancedStaticMesh|SetCustomDataValue _tilevisuals (.InstanceIndex (Utilities|Struct|BreakST_TileDataOLD (Utilities|Array|Get(acopy) (Utilities|Struct|BreakST_TileRowOLD (Utilities|Array|Get(acopy) (Variables|Default|GetGridArray) (LocalVariables|GetGridX))) (LocalVariables|GetGridY)))) 2 _b false)
    (Components|InstancedStaticMesh|SetCustomDataValue _tilevisuals (.InstanceIndex (Utilities|Struct|BreakST_TileDataOLD (Utilities|Array|Get(acopy) (Utilities|Struct|BreakST_TileRowOLD (Utilities|Array|Get(acopy) (Variables|Default|GetGridArray) (LocalVariables|GetGridX))) (LocalVariables|GetGridY)))) 3 _a false)
    (return true)
    (else
      (Development|PrintString "NotWithinTileCords")
      (return false))))