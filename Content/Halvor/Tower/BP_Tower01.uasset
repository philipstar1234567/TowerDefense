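; Tower Blueprint with two counter-rotating torus meshes that grows in through a scale timeline on BeginPlay, then becomes active.
; Tick spins the rings idly until the collision sphere sets an overlapping actor as target, which any end overlap clears.
; With a target, a timeline ramps spin up to maximum, then FireShot runs a delayed cooldown before re-arming.
; The pulse animation is an empty stub and no damage is dealt.
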(event OnComponentBeginOverlap(CollisionSphere)
  (params (OverlappedComponent :type Primitive%20Component%20Object%20Reference) (OtherActor :type Actor%20Object%20Reference) (OtherComp :type Primitive%20Component%20Object%20Reference) (OtherBodyIndex :type Integer) (bFromSweep :type Boolean) (SweepResult :type Hit%20Result%20Structure%20%28by%20ref%29))
  ;[0.15 0.15 0.15 0.5] Enemy Logic
  (Variables|Default|SetTargetActor OtherActor))

(event OnComponentEndOverlap(CollisionSphere)
  (params (OverlappedComponent :type Primitive%20Component%20Object%20Reference) (OtherActor :type Actor%20Object%20Reference) (OtherComp :type Primitive%20Component%20Object%20Reference) (OtherBodyIndex :type Integer))
  ;[0.15 0.15 0.15 0.5] Enemy Logic
  (Variables|Default|SetTargetActor 0))

(event Custom|StartCharge
  (params (Delta%20Seconds :type Float%20%28double-precision%29))
  ;[0.15 0.15 0.15 0.5] Calc Spin Speed
  (Variables|Default|SetbCanShoot false)
  (bind _chargealpha (Timeline|TL_ChargeSpin Play)
    (:Update
      (bind _output_get (Variables|Default|SetSpinSpeedCurrent (Math|Float|Lerp (Variables|Default|GetSpinSpeedIdle) (Variables|Default|GetSpinSpeedMax) _chargealpha)))
      (Transformation|AddLocalRotation (Variables|Default|GetOuterTorusMesh) (Math|Rotator|MakeRotator (* _output_get Delta%20Seconds) 0.0 0.0) false false)
      (Transformation|AddLocalRotation (Variables|Default|GetInnerTorusMesh) (Math|Rotator|MakeRotator (* (* _output_get Delta%20Seconds) -1.0) 0.0 0.0) false false))
    (:Finished
      (CallFunction|FireShot))))

(event Custom|FireShot
  (Variables|Default|SetSpinSpeedCurrent 0.0)
  (CallFunction|PulseAnimation)
  (Utilities|FlowControl|Delay 5.0)
  (Variables|Default|SetSpinSpeedCurrent 5e+01)
  (Utilities|FlowControl|Delay 0.2)
  (Variables|Default|SetbCanShoot true))

(event Custom|PulseAnimation
  ;[0.15 0.15 0.15 0.5] FirePulse Animation
)

(event Custom|DoAttackLogic
  (params (Delta%20Seconds :type Float%20%28double-precision%29))
  (if (Variables|Default|GetbCanShoot)
    (CallFunction|StartCharge Delta%20Seconds)))

(event Custom|DoIdleRotation
  (params (Delta%20Seconds :type Float%20%28double-precision%29))
  (bind _spinspeedidle (Variables|Default|GetSpinSpeedIdle))
  (bind _returnvalue (* Delta%20Seconds _spinspeedidle))
  ;[0.15 0.15 0.15 0.5] Idle Rotation
  (Transformation|AddLocalRotation (Variables|Default|GetOuterTorusMesh) (Math|Rotator|MakeRotator _returnvalue 0.0 0.0) false false)
  (Transformation|AddLocalRotation (Variables|Default|GetInnerTorusMesh) (Math|Rotator|MakeRotator (* _returnvalue -1.0) 0.0 0.0) false false))

(event EventBeginPlay
  ;[0.15 0.15 0.15 0.5] Placement Animation
  (bind _scalealpha (Timeline|TL_PlacementGrow Play)
    (:Update
      (Transformation|SetRelativeScale3D (Variables|Default|GetInnerTorusMesh) (Math|Conversions|ToVector(Float) _scalealpha))
      (Transformation|SetRelativeScale3D (Variables|Default|GetOuterTorusMesh) (Math|Conversions|ToVector(Float) _scalealpha)))
    (:Finished
      (Variables|Default|SetbIsActive true))))

(event EventTick
  (params (DeltaSeconds :type Float%20%28single-precision%29))
  ;[0.15 0.15 0.15 0.5] TickTock
  (if (Variables|Default|GetbIsActive)
    (if (!= (Variables|Default|GetTargetActor) 0)
      (CallFunction|DoAttackLogic DeltaSeconds)
      (else
        (CallFunction|DoIdleRotation DeltaSeconds)))))

(fn ConstructionScript)