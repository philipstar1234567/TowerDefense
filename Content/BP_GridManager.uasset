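; Grid manager actor that builds a tile grid on BeginPlay for world-position lookups and, apparently, placement.
; GenerateGrid fills a nested row array of tile data, offset from the actor, and adds a flattened instanced-mesh visual per tile.
; GetTileFromWorldPosition floors the actor-relative position by tile size and bounds-checks it, returning the tile and a validity flag.
; IsTileValidForPlacement is a stub that always returns false.
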(event Custom|GenerateGrid
  (bind _tilesize (Variables|Default|GetTileSize))
  ;[0.15 0.15 0.15 0.5] Grid Generation System (not a mess at all...)
  (for _index (range 0 (- (Variables|Default|GetGridSizeX) 1))
    (Utilities|Array|Clear (Variables|Default|GetTempRowTiles))
    (for _index_2 (range 0 (- (Variables|Default|GetGridSizeY) 1))
      (Utilities|Array|Add (Variables|Default|GetTempRowTiles) (Utilities|Struct|MakeST_TileData (+ (Math|Vector|MakeVector (* _index _tilesize) (* _tilesize _index_2) 0.0) (Transformation|GetActorLocation)) false (Math|Vector2D|MakeVector2D (Math|Conversions|ToFloat(Integer) _index) (Math|Conversions|ToFloat(Integer) _index_2))))
      (Components|InstancedStaticMesh|AddInstance (Variables|Default|GetTileVisuals) (Math|Transform|MakeTransform (+ (Math|Vector|MakeVector (* _index _tilesize) (* _tilesize _index_2) 0.0) (Transformation|GetActorLocation)) "0, 0, 0" "1.000000,1.000000,0.100000") false))
    (Utilities|Array|Add (Variables|Default|GetGridArray) (Utilities|Struct|MakeST_TileRow (Variables|Default|GetTempRowTiles)))))

(event EventBeginPlay
  ;[0.15 0.15 0.15 0.5] OnBeginPlay
  (Utilities|Array|Clear (Variables|Default|GetGridArray))
  (CallFunction|GenerateGrid))

(fn ConstructionScript)

(fn GetTilefromWorldPosition
  (params (WorldPos :type Vector))
  (bind _returnvalue (Transformation|GetActorLocation))
  (bind _tilesize (Variables|Default|GetTileSize))
  (bind _returnvalue_2 (- WorldPos _returnvalue))
  (bind _returnvalue_3 (/ (.x _returnvalue_2) _tilesize))
  (bind _returnvalue_4 (/ (.y _returnvalue_2) _tilesize))
  (bind _returnvalue_5 (Math|Float|Floor _returnvalue_4))
  (bind _returnvalue_6 (Math|Float|Floor _returnvalue_3))
  (if (and (and (and (>= _returnvalue_6 0) (< _returnvalue_6 (Variables|Default|GetGridSizeX))) (>= _returnvalue_5 0)) (< _returnvalue_5 (Variables|Default|GetGridSizeY)))
    (return (Utilities|Array|Get(acopy) (.rowtiles (Utilities|Array|Get(acopy) (Variables|Default|GetGridArray) _returnvalue_6)) _returnvalue_5) true)
    (else
      (return "" false))))

(fn IsTileValidforPlacement
  (params (GridCoord :type Vector%202D%20Structure))
  (return false))